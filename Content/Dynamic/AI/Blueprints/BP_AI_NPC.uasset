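; AI controller for NPCs that shoot at perceived actors not tagged "Guard".
; On BeginPlay it sets up the PatolData blackboard and runs the BT_AI behavior tree.
; AI Perception updates write a sensed actor to the AimActor key and set Shooting on the controlled Ue4ASP_Character.
; Losing any such actor clears both, with no check that it is the current target.
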(event `self.ReceiveBeginPlay`
  (bind _blackboardcomponent (`self.UseBlackboard` "/Game/Dynamic/AI/Blueprints/PatolData.PatolData"))
  (`self.RunBehaviorTree` "/Game/Dynamic/AI/Blueprints/BT_AI.BT_AI")
  (set `self.BlockboardComp` _blackboardcomponent))

(event `self.AIPerception.OnTargetPerceptionUpdated`
  (params (Actor :type "Actor Object Reference") (Stimulus :type "AIStimulus Structure"))
  (bind _blockboardcomp (`self.BlockboardComp`))
  (bind _asue_4asp_character (cast `/Game/Dynamic/AI/Blueprints/Ue4ASP_Character` (`self.K2_GetPawn`) :!pure true))
  (if (`self.ActorHasTag` Actor "Guard")
    _
    (elif (`.bSuccessfullySensed` (break `AIStimulus` Stimulus))
      (`BlackboardComponent.SetValueAsObject` _blockboardcomp "AimActor" Actor)
      (set `/Game/Dynamic/AI/Blueprints/Ue4ASP_Character.bShooting` true _asue_4asp_character)
      (else
        (`BlackboardComponent.ClearValue` _blockboardcomp "AimActor")
        (set `/Game/Dynamic/AI/Blueprints/Ue4ASP_Character.bShooting` false _asue_4asp_character)))))

(fn `UserConstructionScript`)