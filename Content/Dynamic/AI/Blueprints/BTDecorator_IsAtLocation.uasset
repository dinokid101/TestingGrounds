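; Behavior tree decorator that checks whether the AI pawn is within a set distance of a target actor.
; It reads the target from a blackboard key and passes when the straight-line distance between pawn and target is at most the configured distance.
; It fails when the blackboard actor is not valid.
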(fn `PerformConditionCheckAI`
  (params (OwnerController :type "AIController Object Reference") (ControlledPawn :type "Pawn Object Reference"))
  (returns (ReturnValue :type Boolean))
  (bind _returnvalue (`BTFunctionLibrary.GetBlackboardValueAsActor` (`self.AimActor`)))
  (return (select `bool` (`KismetSystemLibrary.IsValid` _returnvalue) :`true` (<= (`KismetMathLibrary.VSize` (- (`Actor.K2_GetActorLocation` ControlledPawn) (`Actor.K2_GetActorLocation` _returnvalue))) (`self.Distence`)))))