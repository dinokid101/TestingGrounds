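; Level tile for an endlessly spawned path, with a front wall that acts as a gate.
; The player entering LockBox unlocks the wall and, once only, asks BP_GameMode to spawn a tile; leaving it locks the wall.
; Lock and Unlock toggle wall collision and recolor its dynamic material between solid red and translucent green.
; The arrow supplies a spawn transform, and the player touching DestroyBox destroys the tile.
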(event `self.ReceiveBeginPlay`
  (`self.Unlock`))

(event `self.LockBox.OnComponentBeginOverlap`
  (params (OverlappedComponent :type "PrimitiveComponent Object Reference") (OtherActor :type "Actor Object Reference") (OtherComp :type "PrimitiveComponent Object Reference") (OtherBodyIndex :type Integer) (bFromSweep :type Boolean) (SweepResult :type "HitResult Structure (by ref)"))
  (`self.Is Player Actor` OtherActor)
  (`self.Unlock`)
  (`/Engine/EditorBlueprintResources/StandardMacros.DoOnce` false
    (:`Completed`
      (bind _asbp_game_mode (cast `/Game/Dynamic/Levels/BP_GameMode` (`GameplayStatics.GetGameMode`)))
      (`/Game/Dynamic/Levels/BP_GameMode.SpawnTile` _asbp_game_mode))))

(event `self.LockBox.OnComponentEndOverlap`
  (params (OverlappedComponent :type "PrimitiveComponent Object Reference") (OtherActor :type "Actor Object Reference") (OtherComp :type "PrimitiveComponent Object Reference") (OtherBodyIndex :type Integer))
  (`self.Is Player Actor` OtherActor)
  (`self.Lock`))

(event `self.DestroyBox.OnComponentBeginOverlap`
  (params (OverlappedComponent :type "PrimitiveComponent Object Reference") (OtherActor :type "Actor Object Reference") (OtherComp :type "PrimitiveComponent Object Reference") (OtherBodyIndex :type Integer) (bFromSweep :type Boolean) (SweepResult :type "HitResult Structure (by ref)"))
  (`self.Is Player Actor` OtherActor)
  (`self.K2_DestroyActor`))

(fn `GetSpawnTransform`
  (returns (NewTransform :type "Transform Structure"))
  (return (`SceneComponent.K2_GetComponentToWorld` (`self.Arrow`))))

(fn `Lock`
  (bind _frontwall_m (`self.FrontWall_M`))
  (`PrimitiveComponent.SetCollisionEnabled` (`self.FrontWall`) "QueryAndPhysics")
  (`MaterialInstanceDynamic.SetScalarParameterValue` _frontwall_m "Opacity" 1.0)
  (`MaterialInstanceDynamic.SetVectorParameterValue` _frontwall_m "Base Color" (struct :`R` 1.0 :`A` 1.0)))

(fn `Unlock`
  (bind _frontwall_m (`self.FrontWall_M`))
  (`PrimitiveComponent.SetCollisionEnabled` (`self.FrontWall`) "NoCollision")
  (`MaterialInstanceDynamic.SetScalarParameterValue` _frontwall_m "Opacity" 0.5)
  (`MaterialInstanceDynamic.SetVectorParameterValue` _frontwall_m "Base Color" (struct :`G` 1.0 :`A` 1.0)))

(fn `UserConstructionScript`
  (bind _returnvalue (`PrimitiveComponent.CreateDynamicMaterialInstance` (`self.FrontWall`) 0 null))
  (set `self.FrontWall_M` _returnvalue))